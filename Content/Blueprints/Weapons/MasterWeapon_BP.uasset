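; Master weapon Blueprint that handles automatic hitscan firing, ammo tracking and reloading.
; Fire press and release drive a two-gate RetriggerableDelay loop at FireRate, each shot tracing from the camera, playing animation, decrementing ammo and spawning a tracer effect at the hit location.
; Reloads refill the clip from reserve ammo behind timed state flags, triggering automatically on release when empty.
; Trace hits apply no damage, and status messages are debug prints.
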(event Custom|StopFire
  (bind _returnvalue (Game|GetPlayerCameraManager 0))
  (bind _weapondetails (Variables|Default|GetWeaponDetails))
  (bind _returnvalue_2 (Transformation|GetActorLocation _returnvalue))
  ;[1 1 1] Shooting
  (Utilities|FlowControl|Gate true) ; enters at Close
)

(event Custom|StartFire
  (bind _returnvalue (Game|GetPlayerCameraManager 0))
  (bind _weapondetails (Variables|Default|GetWeaponDetails))
  (bind _returnvalue_2 (Transformation|GetActorLocation _returnvalue))
  ;[1 1 1] Shooting
  (Utilities|FlowControl|Sequence
    (:then_0
      (Utilities|FlowControl|Gate false :!label _label
        (:Exit
          (Utilities|FlowControl|Sequence
            (:then_0
              (if (<= (Utilities|Struct|BreakWeaponDetails (Variables|Default|GetWeaponDetails)) 0)
                (Development|PrintString "OUT OF AMMO" true true "(R=1.000000,G=0.078741,B=0.000000,A=1.000000)")
                (Variables|Default|SetCanfire? false)
                (else
                  (bind (_outhit _returnvalue_3) (Collision|LineTraceByChannel _returnvalue_2 (+ _returnvalue_2 (* (Transformation|GetActorForwardVector _returnvalue) 1.5e+04)) "TraceTypeQuery1" false 0 "ForDuration" false))
                  (if _returnvalue_3
                    _
                    (else
                      _))
                  (Variables|Default|SetCanfire? true)
                  (Components|Animation|PlayAnimation (Variables|Default|GetWeaponMesh) (Variables|Default|GetWeaponFireAnim) false)
                  (bind _structout (Utilities|Struct|SetmembersinWeaponDetails _weapondetails (- (.CurrentAmmo (Utilities|Struct|BreakWeaponDetails _weapondetails)) 1)))
                  (Development|PrintString (Utilities|String|ToString(Integer) (Utilities|Struct|BreakWeaponDetails _structout)))
                  (Effects|SpawnEmitteratLocation "/Game/SciFiWeapDark/FX/Particles/P_AssaultRifle_Tracer_Light.P_AssaultRifle_Tracer_Light" (.Location (Collision|BreakHitResult _outhit))))))
            (:then_1
              (goto _label Close))
            (:then_2
              (Utilities|FlowControl|RetriggerableDelay (Variables|Default|GetFireRate))
              (Utilities|FlowControl|Sequence
                (:then_0
                  (goto _label Open))
                (:then_1
                  (Utilities|FlowControl|Gate true :!label _label_2
                    (:Exit
                      (goto _label))))))))))
    (:then_1
      (goto _label_2 Open))))

(event Custom|FirePress
  ;[1 1 1] Reload
  (Variables|Default|SetCanfire? true)
  (if (not (Variables|Default|GetIsReloading?))
    (CallFunction|StartFire)))

(event Custom|FireRelease
  ;[1 1 1] Reload
  (Variables|Default|SetCanfire? false)
  (CallFunction|StopFire)
  (CallFunction|AutoReload))

(event Custom|AutoReload
  ;[1 1 1] Reload
  (if (== (Utilities|Struct|BreakWeaponDetails (Variables|Default|GetWeaponDetails)) 0)
    (if (== (Utilities|Struct|BreakWeaponDetails (Variables|Default|GetWeaponDetails)) 0)
      (Development|PrintString "FIND AMMO" true true "(R=1.000000,G=0.054731,B=0.000000,A=1.000000)")
      (Variables|Default|SetCanfire? false)
      (else
        (Variables|Default|SetIsReloading? true)
        (Variables|Default|SetCanfire? false)
        (CallFunction|Reloading)
        (Utilities|FlowControl|Delay 2.0) ; Reload Animation Time
        (Variables|Default|SetIsReloading? false)
        (Variables|Default|SetCanfire? true)))))

(event Custom|Reloading
  (bind _weapondetails (Variables|Default|GetWeaponDetails))
  (bind (_currentammo _clipsize) (Utilities|Struct|BreakWeaponDetails _weapondetails))
  ;[1 1 1] Reload
  (if (== (Utilities|Struct|BreakWeaponDetails (Variables|Default|GetWeaponDetails)) 0)
    (Development|PrintString "NO AMMO" true true "(R=0.913745,G=1.000000,B=0.192994,A=1.000000)")
    (Variables|Default|SetCanfire? false)
    (elif (== _clipsize _currentammo)
      (Development|PrintString "Magazine Full" true true "(R=0.027826,G=1.000000,B=0.000000,A=1.000000)")
      (Variables|Default|SetCanfire? true)
      (else
        (bind _output_get (Variables|Default|SetIsReloading? true))
        (Variables|Default|SetCanfire? false)
        (if _output_get
          (CallFunction|Reload)
          (Utilities|FlowControl|Delay 2.0) ; Reload Time
          (Variables|Default|SetIsReloading? false)
          (Variables|Default|SetCanfire? true))))))

(event Custom|Reload
  (bind _weapondetails (Variables|Default|GetWeaponDetails))
  (bind _weapondetails_2 (Variables|Default|GetWeaponDetails))
  (bind _weapondetails_3 (Variables|Default|GetWeaponDetails))
  (bind _weapondetails_4 (Variables|Default|GetWeaponDetails))
  (bind _maxammo (Utilities|Struct|BreakWeaponDetails _weapondetails_2))
  (bind (_currentammo _clipsize) (Utilities|Struct|BreakWeaponDetails _weapondetails_3))
  (bind (_currentammo_2 _maxammo_2) (Utilities|Struct|BreakWeaponDetails _weapondetails_4))
  ;[1 1 1] Reload
  (if (not (Variables|Default|GetCanfire?))
    (Components|Animation|PlayAnimation (Variables|Default|GetWeaponMesh) (Variables|Default|GetWeaponReloadAnim) false)
    (if (> (Utilities|Struct|BreakWeaponDetails (Variables|Default|GetWeaponDetails)) 0)
      (Variables|Default|SetNeededAmmo (- _clipsize _currentammo))
      (if (<= _maxammo (Variables|Default|GetNeededAmmo))
        (Utilities|Struct|SetmembersinWeaponDetails _weapondetails (+ _currentammo_2 _maxammo_2))
        (Utilities|Struct|SetmembersinWeaponDetails _weapondetails)
        (else
          (Utilities|Struct|SetmembersinWeaponDetails _weapondetails (- _maxammo (Variables|Default|GetNeededAmmo)))
          (Utilities|Struct|SetmembersinWeaponDetails _weapondetails (Utilities|Struct|BreakWeaponDetails (Variables|Default|GetWeaponDetails))))))))

(fn ConstructionScript
  (Variables|Default|SetWeaponDetails (Utilities|Struct|MakeWeaponDetails (.weapontype (Variables|Default|GetWeaponDetails)) (.damage (Variables|Default|GetWeaponDetails)) (.itemimage (Variables|Default|GetWeaponDetails)) (.currentammo (Variables|Default|GetWeaponDetails)) (.maxammo (Variables|Default|GetWeaponDetails)) (.clipsize (Variables|Default|GetWeaponDetails)))))