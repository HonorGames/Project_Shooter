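; MasterAmmo_BP is an ammo pickup that triggers when a FirstPersonCharacter overlaps its Sphere.
; It stores the character and updates both the WeaponP and WeaponS slots where valid, playing rifle and pistol pickup sounds respectively.
; Each update sets MaxAmmo to CurrentAmmo plus PickupAmmo, rather than adding to the existing MaxAmmo.
; The pickup is never destroyed or disabled here, so every new overlap runs it again.
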(event OnComponentBeginOverlap(Sphere)
  (params (OverlappedComponent :type Primitive%20Component%20Object%20Reference) (OtherActor :type Actor%20Object%20Reference) (OtherComp :type Primitive%20Component%20Object%20Reference) (OtherBodyIndex :type Integer) (bFromSweep :type Boolean) (SweepResult :type Hit%20Result%20Structure%20%28by%20ref%29))
  (bind _asfirst_person_character (Utilities|Casting|CastToFirstPersonCharacter OtherActor))
  (Variables|Default|SetCharRef _asfirst_person_character)
  (CallFunction|AmmoPickup)
  (Development|PrintString "AMMO pickup up function complete"))

(event OnComponentEndOverlap(Sphere)
  (params (OverlappedComponent :type Primitive%20Component%20Object%20Reference) (OtherActor :type Actor%20Object%20Reference) (OtherComp :type Primitive%20Component%20Object%20Reference) (OtherBodyIndex :type Integer))
  (bind _asfirst_person_character (Utilities|Casting|CastToFirstPersonCharacter OtherActor))
  (Variables|Default|SetCharRef _asfirst_person_character))

(event Custom|AmmoPickup
  (bind _charref (Variables|Default|GetCharRef))
  (bind _charref_2 (Variables|Default|GetCharRef))
  (bind _weaponp (Variables|/Game/FirstPersonBP/Blueprints/FirstPersonCharacter.FirstPersonCharacter_C|GetWeaponP _charref_2))
  (bind _weapons (Variables|/Game/FirstPersonBP/Blueprints/FirstPersonCharacter.FirstPersonCharacter_C|GetWeaponS _charref))
  (bind _weapondetails (Variables|/Game/Blueprints/Weapons/MasterWeapon_BP.MasterWeapon_BP_C|GetWeaponDetails _weaponp))
  (bind _weapondetails_2 (Variables|/Game/Blueprints/Weapons/MasterWeapon_BP.MasterWeapon_BP_C|GetWeaponDetails _weapons))
  (if (Utilities|IsValid _weaponp)
    (Utilities|FlowControl|Sequence
      (:then_0
        (Utilities|Struct|SetmembersinWeaponDetails _weapondetails (+ (Variables|Default|GetPickupAmmo) (Utilities|Struct|BreakWeaponDetails _weapondetails)))
        (Audio|PlaySound2D "/Game/SciFiWeapDark/Sound/Rifle/Rifle_AmmoPickup_Cue.Rifle_AmmoPickup_Cue"))
      (:then_1
        (if (Utilities|IsValid _weapons) :!label _label
          (Utilities|Struct|SetmembersinWeaponDetails _weapondetails_2 (+ (Variables|Default|GetPickupAmmo) (Utilities|Struct|BreakWeaponDetails _weapondetails_2)))
          (Audio|PlaySound2D "/Game/SciFiWeapDark/Sound/Pistol/Pistol_AmmoPickup_Cue.Pistol_AmmoPickup_Cue"))))
    (else
      (goto _label))))

(fn ConstructionScript)